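; BP_Flag is a flag pickup that jumps between preset spawn points when a player collects it.
; On the server, a player overlapping its sphere calls GetFlag on that player and picks a new spawn index, with a DoOnce reset next tick.
; A RepNotify on the index moves the flag root to that point.
; SetRandomValue recursively re-rolls to avoid repeats, though its separate random rolls can still repeat.
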(event `self.ReceiveBeginPlay`
  (`/Engine/EditorBlueprintResources/ActorMacros.Switch Has Authority`
    (:`Authority`
      (bind _newrandnum (`self.Set Random Value` (`self.previousRandValue`)))
      (set `self.New Rand Num` _newrandnum))))

(event `self.Sphere.OnComponentBeginOverlap`
  (params (OverlappedComponent :type "PrimitiveComponent Object Reference") (OtherActor :type "Actor Object Reference") (OtherComp :type "PrimitiveComponent Object Reference") (OtherBodyIndex :type Integer) (bFromSweep :type Boolean) (SweepResult :type "HitResult Structure (by ref)"))
  (`/Engine/EditorBlueprintResources/StandardMacros.DoOnce` false :!label _label
    (:`Completed`
      (`KismetSystemLibrary.PrintString` "Collided")
      (bind (_isplayer _playeractor) (message `/Game/Ivan/BPI_Player.IsPlayer` OtherActor))
      (if _isplayer
        (`/Engine/EditorBlueprintResources/ActorMacros.Switch Has Authority`
          (:`Authority`
            (`/Game/Ivan/BP_ThirdPersonCharacter1.GetFlag` _playeractor)
            (bind _newrandnum (`self.Set Random Value` (`self.previousRandValue`)))
            (bind _output_get (set `self.New Rand Num` _newrandnum))
            (`KismetSystemLibrary.PrintString` (`KismetStringLibrary.Concat_StrStr` "Value: " (`KismetStringLibrary.Conv_IntToString` _output_get)))
            (`KismetSystemLibrary.DelayUntilNextTick`)
            (goto _label :!via `Reset`)))))))

(fn `OnRep_New Rand Num`
  (`SceneComponent.K2_SetRelativeLocation` (`self.FlagRoot`) (`|GetArrayItem` (`self.spawnPoints`) (`self.New Rand Num`)) false false))

(fn `Set Random Value`
  (params (prevRandNum :type Integer))
  (returns (newRandNum :type Integer))
  (bind _returnvalue (`KismetMathLibrary.RandomIntegerInRange` 0 (- (`KismetArrayLibrary.Array_Length` (`self.spawnPoints`)) 1)))
  (if (== prevRandNum _returnvalue)
    (bind _newrandnum (`self.Set Random Value` prevRandNum))
    (return _newrandnum)
    (else
      (bind _output_get (set `self.previousRandValue` _returnvalue))
      (return _output_get))))

(fn `UserConstructionScript`)