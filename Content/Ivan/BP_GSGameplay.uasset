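; Game state Blueprint for a timed flag match, showing a countdown, announcing the winner and returning to the Lobby.
; BeginPlay creates the timer widget and sets GameTimer, whose RepNotify refreshes the widgets.
; On authority, that RepNotify also drives the one-second countdown loop until zero triggers EndGame.
; The winner is printed from the highest character FlagCount, numbered by actor array order, before a delayed server travel.
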(event `self.ReceiveBeginPlay`
  (bind _returnvalue (`|CreateWidget` "/Game/Ivan/WBP_MatchTimer.WBP_MatchTimer_C"))
  (`UserWidget.AddToViewport` _returnvalue 0)
  (set `self.gameTimer` 300))

(event `MatchCountdown`
  (`KismetSystemLibrary.Delay` 1.0)
  (set `self.gameTimer` (- (`self.gameTimer`) 1)))

(event `EndGame`
  (`self.DetermineWinner`)
  (`KismetSystemLibrary.Delay` 5.0)
  (`KismetSystemLibrary.ExecuteConsoleCommand` "servertravel Lobby" null))

(fn `DetermineWinner`
  (locals (flagValues :type "Array of Integer"))
  (bind _outactors (`GameplayStatics.GetAllActorsOfClass` "/Game/Ivan/BP_ThirdPersonCharacter1.BP_ThirdPersonCharacter1_C"))
  (for _array_element _outactors
    (`KismetArrayLibrary.Array_Add` (`local.flagValues`) (`/Game/Ivan/BP_ThirdPersonCharacter1.flagCount` _array_element)))
  (`KismetSystemLibrary.PrintString` (`KismetStringLibrary.Concat_StrStr` "Player " (`KismetStringLibrary.Conv_IntToString` (+ (`KismetMathLibrary.MaxOfIntArray` (`local.flagValues`)) 1)) " wins") true true (struct :`R` 0.001526 :`G` 1.0 :`A` 1.0) 7.0))

(fn `OnRep_gameTimer`
  (`self.UpdateCountdownWidget`)
  (`/Engine/EditorBlueprintResources/ActorMacros.Switch Has Authority`
    (:`Authority`
      (if (!= (`self.gameTimer`) 0)
        (`self.MatchCountdown`)
        (else
          (`self.EndGame`))))))

(fn `UpdateCountdownWidget`
  (bind _foundwidgets (`WidgetBlueprintLibrary.GetAllWidgetsOfClass` "/Game/Ivan/WBP_MatchTimer.WBP_MatchTimer_C"))
  (for _array_element _foundwidgets
    (`/Game/Ivan/WBP_MatchTimer.UpdateTimer` _array_element (`self.gameTimer`))))

(fn `UserConstructionScript`)