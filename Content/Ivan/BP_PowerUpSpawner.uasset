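; Power-up spawner actor that, after a random delay from BeginPlay, spawns a random power-up at one of its spawn points.
; The authority waits, then picks a class from PossiblePUClasses and a random SpawnPoints index.
; The actual spawn happens in the index's RepNotify, offsetting the chosen point from the spawner's location, rather than directly in the server event.
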(event `self.ReceiveBeginPlay`
  (`self.DelayBeforeSpawn`))

(event `DelayBeforeSpawn`
  (`/Engine/EditorBlueprintResources/ActorMacros.Switch Has Authority`
    (:`Authority`
      (`KismetSystemLibrary.Delay` (`KismetMathLibrary.RandomFloatInRange` (`self.spawnDelayMin`) (`self.spawnDelayMax`)))
      (`self.SpawnPowerUp`))))

(event `SpawnPowerUp`
  (bind _poweruptospawn (`self.SetRandomPUClass`))
  (set `self.Power Up to Spawn` _poweruptospawn)
  (set `self.spawnPointIndex` (`KismetMathLibrary.RandomIntegerInRange` 0 (`KismetArrayLibrary.Array_LastIndex` (`self.spawnPoints`)))))

(fn `OnRep_NewVar`)

(fn `OnRep_spawnPointIndex`
  (bind _returnvalue (`|SpawnActorFromClass` (`self.Power Up to Spawn`) (`KismetMathLibrary.MakeTransform` (+ (`self.K2_GetActorLocation`) (`|GetArrayItem` (`self.spawnPoints`) (`self.spawnPointIndex`)))) "Undefined" "MultiplyWithRoot" self null)))

(fn `SetRandomPUClass`
  (returns (powerUpToSpawn :type "Actor Class Reference"))
  (return (`|GetArrayItem` (`self.possiblePUClasses`) (`KismetMathLibrary.RandomIntegerInRange` 0 (`KismetArrayLibrary.Array_LastIndex` (`self.possiblePUClasses`))))))

(fn `UserConstructionScript`)