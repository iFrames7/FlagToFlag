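; Speed boost pickup, built on a parent power-up Blueprint, that changes the player's walk speed.
; PowerUp deactivates the pickup's components, saves the player's current MaxWalkSpeed and applies PowerUpWalkSpeed.
; PowerDown restores the saved speed and destroys the actor, with both functions printing debug messages.
; PowerUpEvent only forwards to the parent, and this Blueprint itself never calls PowerUp or PowerDown.
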(event `self.SphereCollider.OnComponentBeginOverlap`
  (params (OverlappedComponent :type "PrimitiveComponent Object Reference") (OtherActor :type "Actor Object Reference") (OtherComp :type "PrimitiveComponent Object Reference") (OtherBodyIndex :type Integer) (bFromSweep :type Boolean) (SweepResult :type "HitResult Structure (by ref)")))

(event `self.PowerUpEvent`
  (params (playerActor :type "/Game/Ivan/BP_ThirdPersonCharacter1 Object Reference"))
  (`parent.PowerUpEvent` playerActor))

(fn `PowerDown`
  (params (playerActor :type "/Game/Ivan/BP_ThirdPersonCharacter1 Object Reference"))
  (set `CharacterMovementComponent.MaxWalkSpeed` (`self.initialMaxWalkSpeed`) (`Character.CharacterMovement` playerActor))
  (`KismetSystemLibrary.PrintString` "Slowing down!")
  (`self.K2_DestroyActor`))

(fn `PowerUp`
  (params (playerActor :type "/Game/Ivan/BP_ThirdPersonCharacter1 Object Reference"))
  (bind _charactermovement (`Character.CharacterMovement` playerActor))
  (`self.DeactivateComponents`)
  (bind _output_get (set `self.initialMaxWalkSpeed` (`CharacterMovementComponent.MaxWalkSpeed` _charactermovement)))
  (`KismetSystemLibrary.PrintString` (`KismetStringLibrary.Conv_DoubleToString` _output_get))
  (set `CharacterMovementComponent.MaxWalkSpeed` (`self.powerUpWalkSpeed`) _charactermovement)
  (`KismetSystemLibrary.PrintString` "Speeding Up!"))

(fn `UserConstructionScript`
  (`parent.UserConstructionScript`))